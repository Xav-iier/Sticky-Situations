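; BP_FadingButton is a button actor that blinks in and out of the level until it is pushed.
; Tick checks the Pushed flag; while false, it uses a Delay and the Active flag to alternate the actor's visibility and collision together.
; Once Pushed is true, Tick keeps the button visible and collidable; this file reads that flag but never sets it.
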(event EventTick
  (params (DeltaSeconds :type Float%20%28single-precision%29))
  ;[0.15 0.15 0.15 0.5] If The Player Has Not Pushed The Button Blink
  (if (Variables|Default|GetPushed)
    (Rendering|SetActorHiddenInGame false)
    (Collision|SetActorEnableCollision true)
    (elif (Variables|Default|GetActive)
      (Utilities|FlowControl|Delay (Variables|Default|GetDelay))
      (Rendering|SetActorHiddenInGame true)
      (Collision|SetActorEnableCollision false)
      (Variables|Default|SetActive false)
      (else
        (Utilities|FlowControl|Delay (Variables|Default|GetDelay))
        (Rendering|SetActorHiddenInGame false)
        (Collision|SetActorEnableCollision true)
        (Variables|Default|SetActive true)))))

(fn ConstructionScript
  (|CallParentFunction))