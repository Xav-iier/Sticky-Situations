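; Checkpoint actor with a flag and pole that updates the player's spawn and grants extra hand throws on touch.
; On overlap with BP_Character, it calls SetSpawn on the character and adds AddThrows to its HandThrows count.
; It then hides itself and disables Flag and Pole collision, retiring the checkpoint without destroying the actor.
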(event Collision|EventActorBeginOverlap
  (params (OtherActor :type Actor%20Object%20Reference))
  (bind _asbp_character (Utilities|Casting|CastToBP_Character OtherActor))
  (Default|SetSpawn _asbp_character)
  (Variables|/Game/Blueprints/BP_Character.BP_Character_C|SetHandThrows _asbp_character (+ (Variables|/Game/Blueprints/BP_Character.BP_Character_C|GetHandThrows _asbp_character) (Variables|Default|GetAddThrows)))
  (Rendering|SetActorHiddenInGame true)
  (Collision|SetCollisionEnabled (Variables|Default|GetFlag) "NoCollision")
  (Collision|SetCollisionEnabled (Variables|Default|GetPole) "NoCollision"))

(fn ConstructionScript)