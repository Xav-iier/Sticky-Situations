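; BP_FallingDebris is a looping hazard that falls from its placed location and costs the player a life on contact.
; A FallDown timeline, triggered from Tick through the GoDown flag, lerps the actor down by Depth without sweeping.
; When it finishes, the debris teleports back to its start with zeroed rotation and re-arms.
; Hits on DebrisCollision call LoseLife on BP_Character, with CanLoseLife and a short delay limiting repeat damage.
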(event OnComponentHit(DebrisCollision)
  (params (HitComponent :type Primitive%20Component%20Object%20Reference) (OtherActor :type Actor%20Object%20Reference) (OtherComp :type Primitive%20Component%20Object%20Reference) (NormalImpulse :type Vector :default "0, 0, 0") (Hit :type Hit%20Result%20Structure%20%28by%20ref%29))
  ;[0.8906 0.781 0 0.5] Deal Damage To The Player Upon Hitting The Debris
  (bind _asbp_character (Utilities|Casting|CastToBP_Character OtherActor))
  (if (Variables|Default|GetCanLoseLife)
    (Default|LoseLife _asbp_character)
    (Variables|Default|SetCanLoseLife false)
    (Utilities|FlowControl|Delay 1.0)
    (Variables|Default|SetCanLoseLife true)))

(event EventBeginPlay
  ;[0 0.8112 0.9062 0.5] Track The Debris Starting Location
  (Variables|Default|SetStartingLocation (Transformation|GetActorLocation)))

(event EventTick
  (params (DeltaSeconds :type Float%20%28single-precision%29))
  ;[0.03037 0.6823 0 0.5] Move The Debris Downwards
  (if (Variables|Default|GetGoDown)
    (bind _falldown (Timeline|FallDown PlayFromStart)
      (:Update
        (Variables|Default|SetGoDown false)
        (Transformation|SetActorLocation (Math|Vector|Lerp(Vector) (Variables|Default|GetStartingLocation) (- (Variables|Default|GetStartingLocation) (Variables|Default|GetDepth)) _falldown) false false))
      (:Finished
        (Transformation|Teleport (Variables|Default|GetStartingLocation) "0, 0, 0")
        (Variables|Default|SetGoDown true)))))

(fn ConstructionScript)