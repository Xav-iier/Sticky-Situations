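; Automatic spring hazard that bobs up and down in a repeating cycle and launches BP_Character straight up on contact while active.
; A timeline started at BeginPlay drives chained MoveComponentTo calls around the starting location, then restarts after a delay; its lerps use a fixed alpha.
; The Active flag is set through both moves and cleared for the pause, gating the Hit launch, which overrides vertical velocity only.
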(event Collision|EventHit
  (params (MyComp :type Primitive%20Component%20Object%20Reference) (Other :type Actor%20Object%20Reference) (OtherComp :type Primitive%20Component%20Object%20Reference) (bSelfMoved :type Boolean) (HitLocation :type Vector :default "0, 0, 0") (HitNormal :type Vector :default "0, 0, 0") (NormalImpulse :type Vector :default "0, 0, 0") (Hit :type Hit%20Result%20Structure%20%28by%20ref%29))
  ;[0.145 0.15 0.02185 0.5] Launch The Player On Contact
  (bind _asbp_character (Utilities|Casting|CastToBP_Character Other))
  (if (Variables|Default|GetActive)
    (Character|LaunchCharacter _asbp_character "0.000000,0.000000,1500.000000" false true)))

(event EventBeginPlay
  ;[0.15 0.03134 0.1307 0.5] Move The Spring Up and Down
  (Variables|Default|SetStartingLocation (Variables|/Script/Engine.SceneComponent|GetRelativeLocation (Variables|Default|GetSpring)))
  (Timeline|Spring%20Platform PlayFromStart
    (:Update
      ;;[0 0 0 0.5] Spring Move Upwards
      (Variables|Default|SetActive true)
      (Components|MoveComponentTo (Variables|Default|GetSpring) (Math|Vector|Lerp(Vector) (Variables|Default|GetStartingLocation) (+ (Variables|Default|GetStartingLocation) "0.000000,0.000000,10.000000") 1.0) "0, 0, 0" false false 0.25 false)
      ;;[0 0 0 0.5] Spring Move Downwards
      (Components|MoveComponentTo (Variables|Default|GetSpring) (Math|Vector|Lerp(Vector) (Variables|Default|GetStartingLocation) (- (Variables|Default|GetStartingLocation) "0.000000,0.000000,10.000000") 1.0) "0, 0, 0" false false 0.5 false)
      (Variables|Default|SetActive false)
      (Utilities|FlowControl|Delay 0.5)
      (Timeline|Spring%20Platform PlayFromStart))))

(fn ConstructionScript)