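; Swinging axe hazard that rocks back and forth along its pitch axis and knocks BP_Character away on contact.
; On BeginPlay it stores its starting rotation, then two Timelines, SwingRight and SwingLeft, restart each other in an endless loop of rotator lerps.
; A Started flag separates the initial half swing from the later full arcs.
; Left and right collision components launch the character with their own velocities.
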(event OnComponentHit(RightCollision)
  (params (HitComponent :type Primitive%20Component%20Object%20Reference) (OtherActor :type Actor%20Object%20Reference) (OtherComp :type Primitive%20Component%20Object%20Reference) (NormalImpulse :type Vector :default "0, 0, 0") (Hit :type Hit%20Result%20Structure%20%28by%20ref%29))
  ;[0.15 0.05078 0.1435 0.5] Launch The Player When Hit By The Axe
  ;;[0 0 0 0.5] Launch The Player To The Right
  (bind _asbp_character (Utilities|Casting|CastToBP_Character OtherActor))
  (Character|LaunchCharacter _asbp_character (Variables|Default|GetRightLaunch) false false))

(event OnComponentHit(LeftCollision)
  (params (HitComponent :type Primitive%20Component%20Object%20Reference) (OtherActor :type Actor%20Object%20Reference) (OtherComp :type Primitive%20Component%20Object%20Reference) (NormalImpulse :type Vector :default "0, 0, 0") (Hit :type Hit%20Result%20Structure%20%28by%20ref%29))
  ;[0.15 0.05078 0.1435 0.5] Launch The Player When Hit By The Axe
  ;;[0 0 0 0.5] Launch The Player Towards The Left
  (bind _asbp_character (Utilities|Casting|CastToBP_Character OtherActor))
  (Character|LaunchCharacter _asbp_character (Variables|Default|GetLeftLaunch) false false))

(event Custom|Swing
  (bind _startingrotation (Variables|Default|GetStartingRotation))
  ;[1 1 1 0.5] Swing Right
  (bind _swing (Timeline|SwingRight PlayFromStart)
    (:Update
      (if (Variables|Default|GetStarted)
        (Transformation|SetActorRotation (Math|Rotator|Lerp(Rotator) (Variables|Default|GetNewRotation) (Math|Rotator|MakeRotator (.roll (Variables|Default|GetNewRotation)) (+ (.pitch (Variables|Default|GetNewRotation)) 8e+01) (.yaw (Variables|Default|GetNewRotation))) _swing))
        (else
          (Transformation|SetActorRotation (Math|Rotator|MakeRotator (.roll (Math|Rotator|Lerp(Rotator) (Variables|Default|GetStartingRotation) (Math|Rotator|MakeRotator (.roll _startingrotation) (+ (.pitch _startingrotation) 4e+01) (.yaw _startingrotation)) _swing)) (.pitch (Math|Rotator|Lerp(Rotator) (Variables|Default|GetStartingRotation) (Math|Rotator|MakeRotator (.roll _startingrotation) (+ (.pitch _startingrotation) 4e+01) (.yaw _startingrotation)) _swing)) (.yaw (Math|Rotator|Lerp(Rotator) (Variables|Default|GetStartingRotation) (Math|Rotator|MakeRotator (.roll _startingrotation) (+ (.pitch _startingrotation) 4e+01) (.yaw _startingrotation)) _swing)))))))
    (:Finished
      (Variables|Default|SetNewRotation (Math|Rotator|Lerp(Rotator) (Variables|Default|GetNewRotation) (Math|Rotator|MakeRotator (.roll (Variables|Default|GetNewRotation)) (+ (.pitch (Variables|Default|GetNewRotation)) 8e+01) (.yaw (Variables|Default|GetNewRotation))) _swing))
      ;[1 1 1 0.5] SwingLeft
      (bind _swing_2 (Timeline|SwingLeft PlayFromStart)
        (:Update
          (if (Variables|Default|GetStarted)
            (Transformation|SetActorRotation (Math|Rotator|Lerp(Rotator) (Variables|Default|GetNewRotation) (Math|Rotator|MakeRotator (.roll (Variables|Default|GetNewRotation)) (- (.pitch (Variables|Default|GetNewRotation)) 8e+01) (.yaw (Variables|Default|GetNewRotation))) _swing_2))
            (else
              (Transformation|SetActorRotation (Math|Rotator|Lerp(Rotator) (Math|Rotator|MakeRotator (.roll (Math|Rotator|Lerp(Rotator) (Variables|Default|GetStartingRotation) (Math|Rotator|MakeRotator (.roll _startingrotation) (+ (.pitch _startingrotation) 4e+01) (.yaw _startingrotation)) _swing)) (.pitch (Math|Rotator|Lerp(Rotator) (Variables|Default|GetStartingRotation) (Math|Rotator|MakeRotator (.roll _startingrotation) (+ (.pitch _startingrotation) 4e+01) (.yaw _startingrotation)) _swing)) (.yaw (Math|Rotator|Lerp(Rotator) (Variables|Default|GetStartingRotation) (Math|Rotator|MakeRotator (.roll _startingrotation) (+ (.pitch _startingrotation) 4e+01) (.yaw _startingrotation)) _swing))) (Math|Rotator|MakeRotator (.roll (Math|Rotator|Lerp(Rotator) (Variables|Default|GetStartingRotation) (Math|Rotator|MakeRotator (.roll _startingrotation) (+ (.pitch _startingrotation) 4e+01) (.yaw _startingrotation)) _swing)) (- (.pitch (Math|Rotator|Lerp(Rotator) (Variables|Default|GetStartingRotation) (Math|Rotator|MakeRotator (.roll _startingrotation) (+ (.pitch _startingrotation) 4e+01) (.yaw _startingrotation)) _swing)) 8e+01) (.yaw (Math|Rotator|Lerp(Rotator) (Variables|Default|GetStartingRotation) (Math|Rotator|MakeRotator (.roll _startingrotation) (+ (.pitch _startingrotation) 4e+01) (.yaw _startingrotation)) _swing))) _swing_2)))))
        (:Finished
          (Variables|Default|SetStarted true)
          (Variables|Default|SetNewRotation (Math|Rotator|Lerp(Rotator) (Math|Rotator|MakeRotator (.roll (Math|Rotator|Lerp(Rotator) (Variables|Default|GetStartingRotation) (Math|Rotator|MakeRotator (.roll _startingrotation) (+ (.pitch _startingrotation) 4e+01) (.yaw _startingrotation)) _swing)) (.pitch (Math|Rotator|Lerp(Rotator) (Variables|Default|GetStartingRotation) (Math|Rotator|MakeRotator (.roll _startingrotation) (+ (.pitch _startingrotation) 4e+01) (.yaw _startingrotation)) _swing)) (.yaw (Math|Rotator|Lerp(Rotator) (Variables|Default|GetStartingRotation) (Math|Rotator|MakeRotator (.roll _startingrotation) (+ (.pitch _startingrotation) 4e+01) (.yaw _startingrotation)) _swing))) (Math|Rotator|MakeRotator (.roll (Math|Rotator|Lerp(Rotator) (Variables|Default|GetStartingRotation) (Math|Rotator|MakeRotator (.roll _startingrotation) (+ (.pitch _startingrotation) 4e+01) (.yaw _startingrotation)) _swing)) (- (.pitch (Math|Rotator|Lerp(Rotator) (Variables|Default|GetStartingRotation) (Math|Rotator|MakeRotator (.roll _startingrotation) (+ (.pitch _startingrotation) 4e+01) (.yaw _startingrotation)) _swing)) 8e+01) (.yaw (Math|Rotator|Lerp(Rotator) (Variables|Default|GetStartingRotation) (Math|Rotator|MakeRotator (.roll _startingrotation) (+ (.pitch _startingrotation) 4e+01) (.yaw _startingrotation)) _swing))) _swing_2))
          (Timeline|SwingRight PlayFromStart))))))

(event EventBeginPlay
  ;[0.15 0.15 0.15 0.5] Set Starting Rotation, and Start Swinging
  (Variables|Default|SetStartingRotation (Transformation|GetActorRotation))
  (CallFunction|Swing))

(fn ConstructionScript)