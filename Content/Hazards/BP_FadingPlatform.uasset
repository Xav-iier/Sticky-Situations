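; Hazard platform that endlessly alternates between solid and vanished on a timed cycle.
; Tick branches on the Active flag, which is true while hidden, into separate Delay nodes for disappearing and reappearing.
; After each delay it toggles actor collision and the Platform component's visibility, then flips the flag.
; The cycle relies on Delay ignoring repeat Tick calls while pending, with no timer or player trigger.
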(event EventTick
  (params (DeltaSeconds :type Float%20%28single-precision%29))
  (if (Variables|Default|GetActive)
    (Utilities|FlowControl|Delay (Variables|Default|GetReappearDelay))
    (Collision|SetActorEnableCollision true)
    (Development|SetHiddeninGame (Variables|Default|GetPlatform) false false)
    (Variables|Default|SetActive false)
    (else
      (Utilities|FlowControl|Delay (Variables|Default|GetDisappear%20Delay))
      (Collision|SetActorEnableCollision false)
      (Development|SetHiddeninGame (Variables|Default|GetPlatform) true false)
      (Variables|Default|SetActive true))))

(fn ConstructionScript)