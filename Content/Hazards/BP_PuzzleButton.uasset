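; Puzzle pressure button that opens a linked door while a character or crate overlaps its trigger box, and closes it when one leaves.
; Overlap events start separate open and close timelines, whose updates call MoveComponentTo to shift the button to a Z offset or back to its stored start location.
; Each timeline's completion then tells the referenced door to open or close.
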(event OnComponentBeginOverlap(Box)
  (params (OverlappedComponent :type Primitive%20Component%20Object%20Reference) (OtherActor :type Actor%20Object%20Reference) (OtherComp :type Primitive%20Component%20Object%20Reference) (OtherBodyIndex :type Integer) (bFromSweep :type Boolean) (SweepResult :type Hit%20Result%20Structure%20%28by%20ref%29))
  (Utilities|Casting|CastToBP_Character OtherActor
    (:then
      (CallFunction|Open))
    (:CastFailed
      (Utilities|Casting|CastToBP_Crate OtherActor)
      (CallFunction|Open))))

(event OnComponentEndOverlap(Box)
  (params (OverlappedComponent :type Primitive%20Component%20Object%20Reference) (OtherActor :type Actor%20Object%20Reference) (OtherComp :type Primitive%20Component%20Object%20Reference) (OtherBodyIndex :type Integer))
  (Utilities|Casting|CastToBP_Character OtherActor
    (:then
      (CallFunction|Close))
    (:CastFailed
      (Utilities|Casting|CastToBP_Crate OtherActor)
      (CallFunction|Close))))

(event Custom|Open
  ;[0.15 0.15 0.15 0.5] Move The Button Down and Open The Door
  (Timeline|OpenDoor PlayFromStart
    (:Update
      (Components|MoveComponentTo (Variables|Default|GetButton) (Math|Vector|Lerp(Vector) (+ (Variables|Default|GetStartLocation) "0.000000,0.000000,100.000000") (Variables|Default|GetStartLocation) 0.0) "0, 0, 0" false false 1.5 false))
    (:Finished
      (Default|DoorOpening (Variables|Default|GetDoor)))))

(event Custom|Close
  ;[0.15 0.15 0.15 0.5] Move The Button Up And Close The Door
  (Timeline|CloseDoor PlayFromStart
    (:Update
      (Components|MoveComponentTo (Variables|Default|GetButton) (Variables|Default|GetStartLocation) "0, 0, 0" false false 1.5 false))
    (:Finished
      (Default|DoorClosing (Variables|Default|GetDoor)))))

(event EventBeginPlay
  ;[0.15 0.15 0.15 0.5] Set Button Location
  (Variables|Default|SetStartLocation (Variables|/Script/Engine.SceneComponent|GetRelativeLocation (Variables|Default|GetButton))))

(fn ConstructionScript)