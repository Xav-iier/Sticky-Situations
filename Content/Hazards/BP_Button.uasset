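; BP_Button is a hazard-folder button that opens a referenced door when the player character hits it.
; BeginPlay stores the button's relative location, and a BP_Character hit sets Pushed and restarts the ButtonMovement timeline.
; Timeline updates call MoveComponentTo with a fixed zero lerp alpha, so the target stays above the start despite the "Move The Button Down" label.
; When the timeline finishes, it calls DoorOpening on DoorReference.
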(event EventBeginPlay
  ;[0.15 0.15 0.15 0.5] Set Button Relative Location
  (Variables|Default|SetStartingLocation (Variables|/Script/Engine.SceneComponent|GetRelativeLocation (Variables|Default|GetButton))))

(event Collision|EventHit
  (params (MyComp :type Primitive%20Component%20Object%20Reference) (Other :type Actor%20Object%20Reference) (OtherComp :type Primitive%20Component%20Object%20Reference) (bSelfMoved :type Boolean) (HitLocation :type Vector :default "0, 0, 0") (HitNormal :type Vector :default "0, 0, 0") (NormalImpulse :type Vector :default "0, 0, 0") (Hit :type Hit%20Result%20Structure%20%28by%20ref%29))
  ;[0.15 0.15 0.15 0.5] Move The Button Down
  (Utilities|Casting|CastToBP_Character Other)
  (Variables|Default|SetPushed true)
  (Timeline|ButtonMovement PlayFromStart
    (:Update
      (Components|MoveComponentTo (Variables|Default|GetButton) (Math|Vector|Lerp(Vector) (+ (Variables|Default|GetStartingLocation) "0.000000,0.000000,100.000000") (Variables|Default|GetStartingLocation) 0.0) "0, 0, 0" false false 1.5 false))
    (:Finished
      (Default|DoorOpening (Variables|Default|GetDoorReference)))))

(fn ConstructionScript)