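; BP_Slingshot is a slingshot hazard actor that detects when a BP_Character enters or leaves its LaunchTrigger volume.
; On overlap begin and end it sets PlayerInside, stores the character reference and calls EnterSlingshot or ExitSlingshot on that character, with a debug print.
; It contains no launch logic of its own and only notifies the character.
; The stored character is not cleared on exit.
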(event OnComponentBeginOverlap(LaunchTrigger)
  (params (OverlappedComponent :type Primitive%20Component%20Object%20Reference) (OtherActor :type Actor%20Object%20Reference) (OtherComp :type Primitive%20Component%20Object%20Reference) (OtherBodyIndex :type Integer) (bFromSweep :type Boolean) (SweepResult :type Hit%20Result%20Structure%20%28by%20ref%29))
  (bind _asbp_character (Utilities|Casting|CastToBP_Character OtherActor))
  (Variables|Default|SetPlayerInside true)
  (bind _output_get (Variables|Default|SetStoredCharacter _asbp_character))
  (Default|EnterSlingshot _output_get)
  (Development|PrintString "Enter slingshot"))

(event OnComponentEndOverlap(LaunchTrigger)
  (params (OverlappedComponent :type Primitive%20Component%20Object%20Reference) (OtherActor :type Actor%20Object%20Reference) (OtherComp :type Primitive%20Component%20Object%20Reference) (OtherBodyIndex :type Integer))
  (bind _asbp_character (Utilities|Casting|CastToBP_Character OtherActor))
  (Variables|Default|SetPlayerInside false)
  (Variables|Default|SetStoredCharacter _asbp_character)
  (Default|ExitSlingshot (Variables|Default|GetStoredCharacter))
  (Development|PrintString "exit slingshot"))

(event EventBeginPlay)

(event Collision|EventActorBeginOverlap
  (params (OtherActor :type Actor%20Object%20Reference)))

(event EventTick
  (params (DeltaSeconds :type Float%20%28single-precision%29)))

(fn ConstructionScript)