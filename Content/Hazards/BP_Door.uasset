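; BP_Door is a hazard door that slides open and shut through DoorOpening and DoorClosing events.
; BeginPlay caches the door's relative location, which opening offsets by MovingSubtraction and closing restores.
; Timelines call MoveComponentTo on each update, with the opening lerp alpha fixed at zero rather than timeline-driven.
; When opening finishes the actor is hidden without collision, and closing restores both before moving.
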(event Custom|DoorOpening
  ;[0.15 0.15 0.15 0.5] Opening Door Animation
  (Timeline|DoorOpen PlayFromStart
    (:Update
      (Components|MoveComponentTo (Variables|Default|GetDoor) (Math|Vector|Lerp(Vector) (- (Variables|Default|GetStartingLocation) (Variables|Default|GetMovingSubtraction)) (Variables|Default|GetStartingLocation) 0.0) "0, 0, 0" false false 2.0 false))
    (:Finished
      (Rendering|SetActorHiddenInGame true)
      (Collision|SetActorEnableCollision false))))

(event Custom|DoorClosing
  ;[0.15 0.15 0.15 0.5] Closing Door Animation
  (Rendering|SetActorHiddenInGame false)
  (Collision|SetActorEnableCollision true)
  (Timeline|DoorClose PlayFromStart
    (:Update
      (Components|MoveComponentTo (Variables|Default|GetDoor) (Variables|Default|GetStartingLocation) "0, 0, 0" false false 2.0 false))))

(event EventBeginPlay
  ;[0.15 0.15 0.15 0.5] Track Door Starting Location
  (Variables|Default|SetStartingLocation (Variables|/Script/Engine.SceneComponent|GetRelativeLocation (Variables|Default|GetDoor))))

(fn ConstructionScript)