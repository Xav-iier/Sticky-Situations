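; BP_AreaGate is a score gate that checks any BP_Character entering its GateTrigger against RequiredScore.
; If the character's MaxScore is too low, it prints a warning with a hardcoded score of 10 and halts the character's movement.
; The SetActorLocation call has no explicit target, so as written it moves the gate itself, not the character, to the character's SpawnLocation.
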(event OnComponentBeginOverlap(GateTrigger)
  (params (OverlappedComponent :type Primitive%20Component%20Object%20Reference) (OtherActor :type Actor%20Object%20Reference) (OtherComp :type Primitive%20Component%20Object%20Reference) (OtherBodyIndex :type Integer) (bFromSweep :type Boolean) (SweepResult :type Hit%20Result%20Structure%20%28by%20ref%29))
  (bind _asbp_character (Utilities|Casting|CastToBP_Character OtherActor))
  (Variables|Default|SetAs%20BP%20Character _asbp_character)
  (if (not (>= (Variables|/Game/Blueprints/BP_Character.BP_Character_C|GetMaxScore _asbp_character) (Variables|Default|GetRequiredScore)))
    (Development|PrintString "You Need 10 Score To Pass!!" true true "(R=1.000000,G=0.000000,B=0.013017,A=1.000000)" 3.0)
    (Transformation|SetActorLocation (Variables|/Game/Blueprints/BP_Character.BP_Character_C|GetSpawnLocation (Variables|Default|GetAs%20BP%20Character)) false false)
    (Components|Movement|StopMovementImmediately (Variables|/Script/Engine.Character|GetCharacterMovement (Variables|Default|GetAs%20BP%20Character)))))

(event EventBeginPlay)

(event Collision|EventActorBeginOverlap
  (params (OtherActor :type Actor%20Object%20Reference)))

(event EventTick
  (params (DeltaSeconds :type Float%20%28single-precision%29)))

(fn ConstructionScript)