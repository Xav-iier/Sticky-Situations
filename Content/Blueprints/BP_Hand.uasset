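; BP_Hand is a sticky hand projectile that stops on overlap and flags the hit on BP_Character.
; On a slime it attaches to the enemy and releases itself after a short delay, clearing the character's swing and hit flags.
; On a crate it attaches the crate to itself, and the GrabCrate timeline, gated by CrateHere, lerps it toward the player.
; Other hits leave it stuck until ReleaseSticky destroys it.
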(event OnComponentBeginOverlap(Hand)
  (params (OverlappedComponent :type Primitive%20Component%20Object%20Reference) (OtherActor :type Actor%20Object%20Reference) (OtherComp :type Primitive%20Component%20Object%20Reference) (OtherBodyIndex :type Integer) (bFromSweep :type Boolean) (SweepResult :type Hit%20Result%20Structure%20%28by%20ref%29))
  (Variables|Default|SetHandLocation (Transformation|GetActorLocation))
  (Variables|Default|SetHandHit true)
  (CallFunction|HandHasHit)
  ;[0.15 0.15 0.15 0.5] Getting attach point of hand
  (Variables|Default|SetAttachPoint (.ImpactPoint (Collision|BreakHitResult SweepResult)))
  (Components|Movement|StopMovementImmediately (Variables|Default|GetProjectileMovement))
  ;[0.15 0.15 0.15 0.5] getting slime cast failed is normal sticking
  (bind _asbp_enemy_slime (Utilities|Casting|CastToBP_Enemy_Slime OtherActor)
    (:then
      ;[0.15 0.15 0.15 0.5] Slime getting rid of hand
      (Transformation|SetActorLocation (Variables|Default|GetAttachPoint) false false)
      (bind _returnvalue (Transformation|AttachActorToActor _asbp_enemy_slime "None" "KeepWorld" "KeepWorld" "KeepWorld" true))
      (Variables|Default|SetbIsAttached _returnvalue)
      (Utilities|FlowControl|Delay 0.75)
      (CallFunction|ReleaseSticky))
    (:CastFailed
      ;[0.15 0.15 0.15 0.5] Pulling Stuff
      (bind _asbp_crate (Utilities|Casting|CastToBP_Crate OtherActor))
      (Variables|Default|SetCrate _asbp_crate)
      (Transformation|SetMobility (Variables|Default|GetHand) "Static")
      (Transformation|AttachComponentToComponent (Variables|Default|GetCrate) (Variables|Default|GetHand) "None" "KeepRelative" "KeepRelative" "KeepWorld" true)
      (if (Variables|/Game/Blueprints/BP_Character.BP_Character_C|GetCrateHere (Variables|Default|GetBP_Character))
        (bind _grabobject (Timeline|GrabCrate Stop)
          (:Update
            (Transformation|SetActorLocation (Math|Vector|Lerp(Vector) (Transformation|GetActorLocation) (Transformation|GetActorLocation (Variables|Default|GetBP_Character)) _grabobject) false false))
          (:Finished
            (Actor|DestroyActor)
            (Variables|/Game/Blueprints/BP_Character.BP_Character_C|SetCrateHere (Variables|Default|GetBP_Character) false)))
        (else
          (Timeline|GrabCrate PlayFromStart))))))

(event Custom|ReleaseSticky
  (bind _bp_character (Variables|Default|GetBP_Character))
  ;[0.15 0.15 0.15 0.5] Release Logic
  (Variables|Default|SetHandHit false)
  (Variables|/Game/Blueprints/BP_Character.BP_Character_C|SetIsSwinging _bp_character false)
  (Variables|/Game/Blueprints/BP_Character.BP_Character_C|SetHandHit _bp_character false)
  (Actor|DestroyActor)
  (Development|PrintString "Destroy"))

(event Custom|HandHasHit
  (bind _output_get (Variables|/Game/Blueprints/BP_Character.BP_Character_C|SetHandHit (Variables|Default|GetBP_Character) true))
  (Development|PrintString (Utilities|String|Append "Hand Hit: " (Utilities|String|ToString(Boolean) _output_get))))

(event EventBeginPlay
  (bind _asbp_character (Utilities|Casting|CastToBP_Character (Game|GetPlayerCharacter 0)))
  (Variables|Default|SetBP_Character _asbp_character))

(fn ConstructionScript)