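; BP_Enemy_DirtThrower is an enemy that throws dirt projectiles and costs the player a life on contact.
; BeginPlay starts a looping timer at ThrowInterval that calls ThrowDirt, which spawns DirtProjectileClass at Arrow1's transform.
; After a throw, a delay runs and then DestroyActor is called on the enemy itself, not the projectile.
; Hit casts the other actor to BP_Character and calls LoseLife.
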(event Custom|ThrowDirt
  (if true
    (bind _returnvalue (Game|SpawnActorfromClass (Variables|Default|GetDirtProjectileClass) (Transformation|GetWorldTransform (Variables|Default|GetArrow1)) "AlwaysSpawn" "MultiplyWithRoot" 0 0))
    (Utilities|FlowControl|Delay 5.0)
    (Actor|DestroyActor)))

(event EventBeginPlay
  (Utilities|Time|SetTimerbyEvent (delegate Custom|ThrowDirt) (Variables|Default|GetThrowInterval) true))

(event Collision|EventHit
  (params (MyComp :type Primitive%20Component%20Object%20Reference) (Other :type Actor%20Object%20Reference) (OtherComp :type Primitive%20Component%20Object%20Reference) (bSelfMoved :type Boolean) (HitLocation :type Vector :default "0, 0, 0") (HitNormal :type Vector :default "0, 0, 0") (NormalImpulse :type Vector :default "0, 0, 0") (Hit :type Hit%20Result%20Structure%20%28by%20ref%29))
  ;[0.15 0.15 0.15 0.5] Damage The Player If They Touch The Enemy
  (bind _asbp_character (Utilities|Casting|CastToBP_Character Other))
  (Default|LoseLife _asbp_character))

(fn ConstructionScript)