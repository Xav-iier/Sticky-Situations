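; BP_CloneEnemy is an enemy that costs the player a life on contact and duplicates itself when the player comes near.
; Its Hit event casts the other actor to BP_Character and calls LoseLife.
; A DetectionSphere overlap with the player spawns another BP_CloneEnemy at a fixed world-space offset.
; A HasCloned flag limits each instance to one clone, with no chain limit visible in the graph.
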(event OnComponentBeginOverlap(DetectionSphere)
  (params (OverlappedComponent :type Primitive%20Component%20Object%20Reference) (OtherActor :type Actor%20Object%20Reference) (OtherComp :type Primitive%20Component%20Object%20Reference) (OtherBodyIndex :type Integer) (bFromSweep :type Boolean) (SweepResult :type Hit%20Result%20Structure%20%28by%20ref%29))
  ;[0.15 0.15 0.15 0.5] Cloning
  (Utilities|Casting|CastToBP_Character OtherActor)
  (if (not (Variables|Default|GetHasCloned))
    (Variables|Default|SetHasCloned true)
    (Game|SpawnActorfromClass "BP_CloneEnemy_C" (Math|Transform|MakeTransform (+ (Transformation|GetActorLocation) (Math|Vector|MakeVector 17.0 2e+02 0.0))) "Undefined" "MultiplyWithRoot" 0 0)))

(event Collision|EventHit
  (params (MyComp :type Primitive%20Component%20Object%20Reference) (Other :type Actor%20Object%20Reference) (OtherComp :type Primitive%20Component%20Object%20Reference) (bSelfMoved :type Boolean) (HitLocation :type Vector :default "0, 0, 0") (HitNormal :type Vector :default "0, 0, 0") (NormalImpulse :type Vector :default "0, 0, 0") (Hit :type Hit%20Result%20Structure%20%28by%20ref%29))
  ;[0.15 0.15 0.15 0.5] Damage The Player If They Touch The Enemy
  (bind _asbp_character (Utilities|Casting|CastToBP_Character Other))
  (Default|LoseLife _asbp_character))

(fn ConstructionScript)